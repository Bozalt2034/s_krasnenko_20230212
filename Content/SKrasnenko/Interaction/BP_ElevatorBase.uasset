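; Base elevator actor that moves a platform along a spline in response to an interaction.
; It extends the parent's ActivateInteract, then plays the MovinScale timeline when OnActive is true and reverses it otherwise.
; Each timeline update samples the spline by time to set the platform's world location, taking only the yaw from the spline rotation so the platform stays level.
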(event `self.ActivateInteract`
  (params (ActivateInteract :type Boolean))
  ;[1 1 1] Перегрузка родительской функции
  (`parent.ActivateInteract` ActivateInteract)
  (if (`self.OnActive`)
    ;[1 1 1] Таймлайн движения лифта
    (bind (_direction _movingscale) (`Timeline|MovinScale` :!label _label)
      (:`Update`
        ;[1 1 1] Обновляет лока платформы в мировых координатах, при этом берет конкретную точку сплайна
        (`SceneComponent.K2_SetWorldLocation` (`self.Platform`) (`SplineComponent.GetLocationAtTime` (`self.Spline`) _movingscale "World" false) false false)
        (`SceneComponent.K2_SetWorldRotation` (`self.Platform`) (`KismetMathLibrary.MakeRotator` 0.0 0.0 (.yaw (`SplineComponent.GetRotationAtTime` (`self.Spline`) _movingscale "World" false))) false false)))
    (else
      (goto _label :!via `Reverse`))))

(fn `UserConstructionScript`
  (`parent.UserConstructionScript`))