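; BP_LaserGun is a laser weapon that deals continuous damage along a beam while firing.
; An overridden Fire event toggles LaserActive.
; While active, Tick line-traces from the Arrow along its forward vector for AtacRange against WorldStatic and Pawn objects, drawn as a one-frame debug line.
; On a hit it moves spark particles to the impact point and applies Damage scaled by delta seconds; otherwise the particles deactivate.
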(event `self.Fire`
  (params (ActivateGun :type Boolean))
  ;[1 1 1] Перегрузка базовой функции
  (set `self.LaserActive` ActivateGun))

(event `self.ReceiveTick`
  (params (DeltaSeconds :type "Float (single-precision)"))
  (bind _arrow (`self.Arrow`))
  (bind _particlesystem (`self.ParticleSystem`))
  (bind _returnvalue (`SceneComponent.K2_GetComponentLocation` _arrow))
  (if (`self.LaserActive`)
    ;[1 1 1] Определяет с чем произошло столкновение
    (bind (_outhit _returnvalue_2) (`KismetSystemLibrary.LineTraceSingleForObjects` :`Start` _returnvalue :`End` (+ _returnvalue (* (`SceneComponent.GetForwardVector` _arrow) (`self.AtacRange`))) :`ObjectTypes` (`|MakeArray` "ObjectTypeQuery1" "ObjectTypeQuery3" :!type "EObjectTypeQuery Enum") :`DrawDebugType` "ForOneFrame"))
    ;[1 1 1] Активация/деактивация partical эффекта
    (if _returnvalue_2
      (`ActorComponent.Activate` _particlesystem false)
      (bind (_bblockinghit _binitialoverlap _time _distance _location _impactpoint _normal _impactnormal _physmat _hitactor) (`GameplayStatics.BreakHitResult` _outhit))
      ;[1 1 1] Изменениея координат искр, взависимости от точки попадания
      (`SceneComponent.K2_SetWorldLocation` (`self.ParticleSystem`) _impactpoint false false)
      ;[1 1 1] Нанесение урона объекту попавшему под луч
      (`GameplayStatics.ApplyDamage` _hitactor (* (`self.Damage`) (`GameplayStatics.GetWorldDeltaSeconds`)) null self)
      (else
        (`ActorComponent.Deactivate` _particlesystem)))
    (else
      ;[1 1 1] Отключает partical эффект
      (`ActorComponent.Deactivate` (`self.ParticleSystem`)))))

(fn `UserConstructionScript`
  (`parent.UserConstructionScript`))